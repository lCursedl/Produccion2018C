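; Game mode for ShellShocked, a local multiplayer tank game with a countdown timer widget.
; On BeginPlay it spawns and possesses a tank per local player, matching PlayerStart tags to player indices.
; Tick uses a one-second Delay to count down Secs.
; At zero it disables tank input and collects survivors with health left, but the multiple-survivor check leads to no action.
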(event EventBeginPlay
  (CallFunction|GetPlayerStartPoints)
  (CallFunction|SpawnPlayers)
  (bind _returnvalue (UserInterface|CreateWidget "/Game/Timer.Timer_C"))
  (UserInterface|Viewport|AddtoViewport _returnvalue 0))

(event EventTick
  (params (DeltaSeconds :type Float%20%28single-precision%29))
  (if (<= (Variables|Default|GetSecs) 0)
    (for _array_element (Variables|Default|GetPlayers)
      (Input|DisableInput _array_element 0)
      (if (> (Default|GetHealth _array_element) 0)
        (Utilities|Array|Add (Variables|Default|GetCheckedPlayers) _array_element)))
    (if (> (Utilities|Array|Length (Variables|Default|GetCheckedPlayers)) 1)
      _)
    (else
      (Utilities|FlowControl|Delay 1.0)
      (Math|Integer|DecrementInt (Variables|Default|GetSecs)))))

(fn ConstructionScript)

(fn GetPlayerStartPoints
  (bind _outactors (Actor|GetAllActorsOfClass "/Script/Engine.PlayerStart"))
  (Variables|Default|SetPlayer%20Start%20Array _outactors))

(fn SpawnPlayers
  (for _index (range 0 (- (Variables|Default|GetMaxPlayerCount) 1))
    (Variables|Default|SetIndex _index)
    (for _array_element (Variables|Default|GetPlayer%20Start%20Array)
      (if (Utilities|Name|Equal(Name) (Variables|/Script/Engine.PlayerStart|GetPlayerStartTag _array_element) (Utilities|String|StringToName (Utilities|String|ToString(Integer) (Variables|Default|GetIndex))))
        (Class|GameplayStatics|CreatePlayer (Variables|Default|GetIndex))
        (bind _returnvalue (Game|SpawnActorfromClass "/Game/Player/Tank.Tank_C" (Transformation|GetActorTransform _array_element) "Undefined" 0 0))
        (Default|RotateBox _returnvalue (Transformation|GetActorRotation _array_element))
        (Pawn|Possess (Game|GetPlayerController (Variables|Default|GetIndex)) _returnvalue)
        (Utilities|Array|Add (Variables|Default|GetPlayers) _returnvalue)))))