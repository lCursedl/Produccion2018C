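; BP_Model is a pickup actor that adds points to the third-person player when overlapped.
; On BeginPlay it caches the player character, loops over all BP_ModelSpawner actors, keeps the last as its spawner reference and scales itself to quarter size.
; Any actor overlap, with no check on the other actor, awards its Points to that cached player, decrements the spawner's CurrentSpawn and destroys the pickup.
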(event EventBeginPlay
  (bind _asthird_person_character (Utilities|Casting|CastToThirdPersonCharacter (Game|GetPlayerCharacter 0)))
  (Variables|Default|SetPlayer _asthird_person_character)
  (bind _outactors (Actor|GetAllActorsOfClass "/Game/BPs/Spawns/BP_ModelSpawner.BP_ModelSpawner_C"))
  (for _array_element _outactors
    (Variables|Default|SetSpawn%20Reference _array_element)
    (Transformation|SetActorScale3D "0.250000,0.250000,0.250000")))

(event Collision|EventActorBeginOverlap
  (params (OtherActor :type Actor%20Object%20Reference))
  (bind _player (Variables|Default|GetPlayer))
  (Variables|/Game/ThirdPersonCPP/Blueprints/ThirdPersonCharacter.ThirdPersonCharacter_C|SetPoints _player (+ (Variables|/Game/ThirdPersonCPP/Blueprints/ThirdPersonCharacter.ThirdPersonCharacter_C|GetPoints _player) (Variables|Default|GetPoints)))
  (Math|Integer|DecrementInt (Variables|/Game/BPs/Spawns/BP_ModelSpawner.BP_ModelSpawner_C|GetCurrent%20Spawn (Variables|Default|GetSpawn%20Reference))
    (:%20%20
      (Actor|DestroyActor))))

(event EventTick
  (params (DeltaSeconds :type Float%20%28single-precision%29)))

(fn ConstructionScript)