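; BP_ModelSpawner is a spawner actor that places BP_Model actors at random spots until a spawn limit is reached.
; Tick checks CurrentSpawn against MaxSpawn and runs a Delay of SpawnTime, which paces the spawns.
; Each spawn uses a random X and Y at a fixed height in world space, independent of the spawner's location, then increments CurrentSpawn.
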(event EventBeginPlay)

(event Collision|EventActorBeginOverlap
  (params (OtherActor :type Actor%20Object%20Reference)))

(event EventTick
  (params (DeltaSeconds :type Float%20%28single-precision%29))
  (if (< (Variables|Default|GetCurrent%20Spawn) (Variables|Default|GetMaxSpawn))
    (Utilities|FlowControl|Delay (Variables|Default|GetSpawn%20Time))
    (Game|SpawnActorfromClass "/Game/BPs/Actors/BP_Model.BP_Model_C" (Math|Conversions|ToTransform(Vector) (Math|Vector|MakeVector (Math|Conversions|ToFloat(Integer) (Math|Random|RandomIntegerinRange -500 1000)) (Math|Conversions|ToFloat(Integer) (Math|Random|RandomIntegerinRange -500 500)) 2.5e+02)) "Undefined" 0 0)
    (Math|Integer|IncrementInt (Variables|Default|GetCurrent%20Spawn))))

(fn ConstructionScript)